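; Turret actor for a multiplayer ship game, currently an unfinished prototype of server-side proximity detection with no aiming or firing.
; When an actor begins overlapping its sphere, the authority measures the distance with a vector-length helper and briefly prints the actor's name if it is within a fixed range.
; Tick also runs a GetAllActorsOfClass search on the authority every frame, but the loop over the results does nothing.
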(event OnComponentBeginOverlap(Sphere)
  (params (OtherActor :type Actor%20Object%20Reference) (OtherComp :type Primitive%20Component%20Object%20Reference) (OtherBodyIndex :type Integer) (bFromSweep :type Boolean) (SweepResult :type Hit%20Result%20Structure%20%28by%20ref%29))
  (Networking|SwitchHasAuthority
    (:Authority
      (bind _distance (CallFunction|Distance (Transformation|GetActorLocation OtherActor) (Transformation|GetActorLocation)))
      (if (< _distance 1.5e+03)
        (Development|PrintString (Utilities|GetDisplayName OtherActor) true true "(R=0.000000,G=0.660000,B=1.000000,A=1.000000)" 0.5)))))

(event EventBeginPlay)

(event EventActorBeginOverlap
  (params (OtherActor :type Actor%20Object%20Reference)))

(event EventTick
  (params (DeltaSeconds :type Float%20%28single-precision%29)))

(event EventTick
  (params (DeltaSeconds :type Float%20%28single-precision%29))
  (Networking|SwitchHasAuthority
    (:Authority
      (bind _outactors (Actor|GetAllActorsOfClass 0))
      (for _array_element _outactors
        _))))

(fn ConstructionScript)

(fn Distance
  (params (Actor%201 :type Vector) (Actor%202 :type Vector))
  (return (Math|Vector|VectorLength (- Actor%201 Actor%202))))