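; Player controller for the multiplayer ship game that maps input to PlayerShip actions.
; It finds the ship through player index 0 lookups, then toggles its MainMenu visibility or calls AttemptFire to fire the laser.
; Forward input adds movement along the controlled pawn's forward vector, while positive left and right rotation input calls the ship's ServerRotate with a fixed signed step.
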(event EventBeginPlay)

(event EventTick
  (params (DeltaSeconds :type Float%20%28single-precision%29)))

(event Input|ActionEvents|InputActionFire
  (params (Key :type Key%20Structure :default "AnyKey"))
  ;[1 1 1] Fire laser
  (:Pressed
    (bind _asplayer_ship (Utilities|Casting|CastToPlayerShip (Game|GetPlayerCharacter 0)))
    (Utilities|IsValid _asplayer_ship
      (:Is%20Valid
        (Default|AttemptFire _asplayer_ship _asplayer_ship)))))

(event Input|ActionEvents|InputActionMenu
  (params (Key :type Key%20Structure :default "AnyKey"))
  (:Pressed
    (bind _asplayer_ship (Utilities|Casting|CastToPlayerShip (Game|GetPlayerCharacter 0)))
    (switch Utilities|FlowControl|Switch|SwitchonESlateVisibility (Widget|GetVisibility (Variables|/Game/MultiplayerShip/Blueprints/PlayerShip/PlayerShip.PlayerShip_C|GetMainMenu _asplayer_ship))
      (:Visible
        (Widget|SetVisibility (Variables|/Game/MultiplayerShip/Blueprints/PlayerShip/PlayerShip.PlayerShip_C|GetMainMenu _asplayer_ship) "Hidden"))
      (:Hidden
        (Widget|SetVisibility (Variables|/Game/MultiplayerShip/Blueprints/PlayerShip/PlayerShip.PlayerShip_C|GetMainMenu _asplayer_ship) "Visible")))))

(event Input|AxisEvents|InputAxisRotateLeft
  (params (AxisValue :type Float%20%28single-precision%29))
  ;[1 1 1] Rotate Left
  (if (> AxisValue 0.0)
    (bind _asplayer_ship (Utilities|Casting|CastToPlayerShip (Game|GetPlayerCharacter 0)))
    (Default|ServerRotate _asplayer_ship _asplayer_ship -5.0)))

(event Input|AxisEvents|InputAxisRotateRight
  (params (AxisValue :type Float%20%28single-precision%29))
  ;[1 1 1] Rotate Right
  (if (> AxisValue 0.0)
    (bind _asplayer_ship (Utilities|Casting|CastToPlayerShip (Game|GetPlayerCharacter 0)))
    (Default|ServerRotate _asplayer_ship _asplayer_ship 5.0)))

(event Input|AxisEvents|InputAxisForward
  (params (AxisValue :type Float%20%28single-precision%29))
  (bind _returnvalue (Game|GetPlayerController 0))
  (bind _returnvalue_2 (Pawn|GetControlledPawn _returnvalue))
  ;[1 1 1] Forward movement
  (Utilities|IsValid _returnvalue_2
    (:Is%20Valid
      (Pawn|Input|AddMovementInput _returnvalue_2 (Transformation|GetActorForwardVector _returnvalue_2) AxisValue false))))

(fn ConstructionScript)