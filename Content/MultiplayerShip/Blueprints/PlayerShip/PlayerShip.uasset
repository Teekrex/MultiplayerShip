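; Player ship for a multiplayer flag game, with energy-limited lasers, health, team and flag dropping.
; Authority-gated events handle rotation, laser spawning, damage from laser overlaps and energy regeneration, with a RepNotify applying the replicated yaw.
; Tick also drives every MiniMap actor.
; BeginPlay initializes attributes and creates main menu and ship HUD widgets, whose visibility ChangeState swaps.
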(event OnComponentBeginOverlap(Box)
  (params (OtherActor :type Actor%20Object%20Reference) (OtherComp :type Primitive%20Component%20Object%20Reference) (OtherBodyIndex :type Integer) (bFromSweep :type Boolean) (SweepResult :type Hit%20Result%20Structure%20%28by%20ref%29))
  ;[1 1 1] Laser collision with ships
  (Networking|SwitchHasAuthority
    (:Authority
      (bind _asship_laser (Utilities|Casting|CastToShipLaser OtherActor))
      (CallFunction|TakeDamage 1.0))))

(event Custom|ServerRotate
  (params (RotatingShip :type Player%20Ship%20Object%20Reference) (Direction :type Float%20%28single-precision%29))
  ;[1 1 1] Rotate on server
  (Networking|SwitchHasAuthority
    (:Authority
      (Variables|Default|SetRotation (+ (.Yaw (Math|Rotator|BreakRotator (Transformation|GetActorRotation RotatingShip))) Direction)))))

(event Custom|DropFlag
  ;[1 1 1] Drop flag
  (bind _asship_game_state (Utilities|Casting|CastToShipGameState (Game|GetGameState)))
  (Default|DropFlag (Variables|/Game/MultiplayerShip/Blueprints/ShipGameState.ShipGameState_C|GetTheFlag _asship_game_state)))

(event Custom|JoinTeam
  (Networking|SwitchHasAuthority
    (:Authority
      (Variables|Default|SetTeam 2))))

(event Custom|AttemptFire
  (params (Ship :type Player%20Ship%20Object%20Reference))
  (bind _returnvalue (Transformation|GetActorRotation Ship))
  ;[1 1 1] Fire on server
  (if (> (Variables|PlayerShip_C|GetEnergy Ship) 0.0)
    (Networking|SwitchHasAuthority
      (:Authority
        (Variables|Default|SetEnergy (- (Variables|Default|GetEnergy) 1.0))
        (bind _returnvalue_2 (Game|SpawnActorfromClass "/Game/MultiplayerShip/Blueprints/PlayerShip/ShipLaser.ShipLaser_C" (Math|Transform|MakeTransform (+ (Transformation|GetActorLocation Ship) (* (Math|Vector|GetForwardVector _returnvalue) 1e+02)) _returnvalue) "Undefined" 0 0))
        (Variables|/Game/MultiplayerShip/Blueprints/PlayerShip/ShipLaser.ShipLaser_C|SetShipOwner _returnvalue_2 self)))))

(event EventBeginPlay)

(event EventActorBeginOverlap
  (params (OtherActor :type Actor%20Object%20Reference)))

(event EventTick
  (params (DeltaSeconds :type Float%20%28single-precision%29)))

(event EventBeginPlay
  ;[1 1 1] Init HUD and attributes
  (CallFunction|InitAttributes)
  (CallFunction|InitHUD))

(event EventTick
  (params (DeltaSeconds :type Float%20%28single-precision%29))
  ;[1 1 1] update mini map
  (bind _outactors (Actor|GetAllActorsOfClass "/Game/MultiplayerShip/Blueprints/MiniMap/MiniMap.MiniMap_C"))
  (for _array_element _outactors
    (Default|OutsideTick _array_element)
    ;[1 1 1] Update energy every second
    (Networking|SwitchHasAuthority
      (:Authority
        (Utilities|FlowControl|Delay 1.0)
        (Variables|Default|SetEnergy (Math|Float|Clamp(Float) (+ (Variables|Default|GetEnergy) 1.0) 0.0 (Variables|Default|GetMaxEnergy)))))))

(event Input|ActionEvents|InputActionAction
  (params (Key :type Key%20Structure :default "AnyKey"))
  (:Pressed
    (CallFunction|DropFlag)))

(fn ConstructionScript)

(fn OnRepRotation
  (bind _returnvalue (Game|Player|GetPlayerPawn 0))
  (bind _returnvalue_2 (Transformation|GetActorRotation _returnvalue))
  (bind (_roll _pitch) (Math|Rotator|BreakRotator _returnvalue_2))
  (Utilities|IsValid _returnvalue
    (:Is%20Valid
      (Transformation|SetActorRotation (Math|Rotator|MakeRotator _roll _pitch (Variables|Default|GetRotation))))))

(fn InitAttributes
  (Networking|SwitchHasAuthority
    (:Authority
      (Variables|Default|SetEnergy (Variables|Default|GetMaxEnergy))
      (Variables|Default|SetHealth (Variables|Default|GetMaxHealth)))))

(fn TakeDamage
  (params (Damage :type Float%20%28single-precision%29))
  (Networking|SwitchHasAuthority
    (:Authority
      (if (not (Variables|Default|GetInvuln))
        (Variables|Default|SetHealth (- (Variables|Default|GetHealth) 1.0))))))

(fn InitHUD
  (bind _returnvalue (Game|GetPlayerController 0))
  (bind _returnvalue_2 (UserInterface|CreateWidget "/Game/MultiplayerShip/Blueprints/MainMenu.MainMenu_C" _returnvalue))
  (UserInterface|Viewport|AddtoViewport _returnvalue_2 0)
  (bind _output_get (Variables|Default|SetMainMenu _returnvalue_2))
  (Widget|SetVisibility _output_get "Visible")
  (bind _returnvalue_3 (UserInterface|CreateWidget "/Game/MultiplayerShip/Blueprints/ShipHud.ShipHud_C" _returnvalue))
  (bind _output_get_2 (Variables|Default|SetMyHud _returnvalue_3))
  (UserInterface|Viewport|AddtoViewport _output_get_2 0)
  (Widget|SetVisibility _output_get_2 "Hidden"))

(fn ChangeState
  (params (State :type Integer))
  (switch int State
    (:0
      (Widget|SetVisibility (Variables|Default|GetMyHud) "Hidden")
      (Widget|SetVisibility (Variables|Default|GetMainMenu) "Visible"))
    (:1
      (Widget|SetVisibility (Variables|Default|GetMyHud) "Visible")
      (Widget|SetVisibility (Variables|Default|GetMainMenu) "Hidden"))))