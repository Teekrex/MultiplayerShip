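; Capture-the-flag pickup actor for multiplayer ship matches, carried by player ships and returned home on scoring.
; On the authority, sphere overlap records the holder and flag in ShipGameState, then attaches it to a PlayerShip's FlagSocket.
; Pickup requires over two seconds since dropping, measured using only the clock's seconds component, which wraps each minute.
; ReturnHome reports the score to CTFGameMode, calls DropFlag to clear the holder and detach, then moves to FlagHome.
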(event OnComponentBeginOverlap(Sphere)
  (params (OtherActor :type Actor%20Object%20Reference) (OtherComp :type Primitive%20Component%20Object%20Reference) (OtherBodyIndex :type Integer) (bFromSweep :type Boolean) (SweepResult :type Hit%20Result%20Structure%20%28by%20ref%29))
  (Networking|SwitchHasAuthority
    (:Authority
      (if (> (- (Class|KismetMathLibrary|GetSecond (Math|DateTime|Now)) (Variables|Default|GetLastDropped)) 2)
        (Networking|SwitchHasAuthority
          (:Authority
            (bind _asship_game_state (Utilities|Casting|CastToShipGameState (Game|GetGameState)))
            (Variables|/Game/MultiplayerShip/Blueprints/ShipGameState.ShipGameState_C|SetWhoHasFlag _asship_game_state (Utilities|GetDisplayName OtherActor))
            (Variables|/Game/MultiplayerShip/Blueprints/ShipGameState.ShipGameState_C|SetTheFlag _asship_game_state self)
            (bind _asplayer_ship (Utilities|Casting|CastToPlayerShip OtherActor))
            (Class|Actor|AttachRootComponentto (Variables|/Script/Engine.Character|GetMesh _asplayer_ship) "FlagSocket" "SnapToTarget" true)))))))

(event EventBeginPlay)

(event EventActorBeginOverlap
  (params (OtherActor :type Actor%20Object%20Reference)))

(event EventTick
  (params (DeltaSeconds :type Float%20%28single-precision%29)))

(fn ConstructionScript)

(fn DropFlag
  (bind _asship_game_state (Utilities|Casting|CastToShipGameState (Game|GetGameState)))
  (Variables|/Game/MultiplayerShip/Blueprints/ShipGameState.ShipGameState_C|SetWhoHasFlag _asship_game_state "None")
  (Variables|Default|SetLastDropped (Class|KismetMathLibrary|GetSecond (Math|DateTime|Now)))
  (Class|Actor|DetachRootComponentfromParent true))

(fn ReturnHome
  (params (ScoringTeam :type Integer))
  (bind _asctfgame_mode (Utilities|Casting|CastToCTFGameMode (Game|GetGameMode)))
  (Default|TeamScore _asctfgame_mode ScoringTeam)
  (CallFunction|DropFlag)
  (Transformation|SetActorLocation (Transformation|GetActorLocation (Variables|Default|GetFlagHome)) false false))