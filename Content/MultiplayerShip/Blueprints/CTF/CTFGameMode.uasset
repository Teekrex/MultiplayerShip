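; CTFGameMode is the game mode for Capture the Flag in the multiplayer ship game, handling team scoring.
; TeamScore runs only with authority, casts the game state to ShipGameState and adds one point to Team1Score or Team2Score based on the Team argument.
; Each score also prints a debug message, and the event graph holds only disabled placeholder events.
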(event EventBeginPlay
  (|CallParentFunction))

(event EventTick
  (params (DeltaSeconds :type Float%20%28single-precision%29))
  (|CallParentFunction 0.0))

(fn ConstructionScript
  (|CallParentFunction))

(fn TeamScore
  (params (Team :type Integer))
  (Networking|SwitchHasAuthority
    (:Authority
      (bind _asship_game_state (Utilities|Casting|CastToShipGameState (Game|GetGameState)))
      (switch int Team
        (:1
          (Variables|/Game/MultiplayerShip/Blueprints/ShipGameState.ShipGameState_C|SetTeam1Score _asship_game_state (+ (Variables|/Game/MultiplayerShip/Blueprints/ShipGameState.ShipGameState_C|GetTeam1Score _asship_game_state) 1)))
        (:2
          (Variables|/Game/MultiplayerShip/Blueprints/ShipGameState.ShipGameState_C|SetTeam2Score _asship_game_state (+ (Variables|/Game/MultiplayerShip/Blueprints/ShipGameState.ShipGameState_C|GetTeam2Score _asship_game_state) 1))))
      (Development|PrintString "Score!"))))