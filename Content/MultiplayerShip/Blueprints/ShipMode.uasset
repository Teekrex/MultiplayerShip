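; ShipMode is the game mode for a multiplayer ship game, handling ship death and respawn on the server.
; BeginPlay caches all PlayerStart actors, while Tick polls every PlayerShip and triggers Respawn when health drops below 1.
; Respawn retries random start selection until valid, since the index range can overrun the array, then waits briefly, teleports the ship and reinitializes its attributes.
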(event Custom|Respawn
  (params (PlayerShip :type Player%20Ship%20Object%20Reference))
  ;[1 1 1] Respawn ship
  (Variables|Default|SetPlayerShip PlayerShip)
  (Networking|SwitchHasAuthority
    (:Authority
      (bind _playerstart (CallFunction|GetRandomStart :!label _label))
      (Utilities|IsValid _playerstart
        (:Is%20Valid
          (Utilities|FlowControl|Delay 2.0)
          (Transformation|Teleport (Variables|Default|GetPlayerShip) (Transformation|GetActorLocation _playerstart) "0, 0, 0")
          (Default|InitAttributes (Variables|Default|GetPlayerShip)))
        (:Is%20Not%20Valid
          (goto _label))))))

(event EventBeginPlay)

(event EventTick
  (params (DeltaSeconds :type Float%20%28single-precision%29)))

(event EventTick
  (params (DeltaSeconds :type Float%20%28single-precision%29))
  ;[1 1 1] Check  if ships are dead
  (Networking|SwitchHasAuthority
    (:Authority
      (bind _outactors (Actor|GetAllActorsOfClass "/Game/MultiplayerShip/Blueprints/PlayerShip/PlayerShip.PlayerShip_C"))
      (for _array_element _outactors
        (bind _asplayer_ship (Utilities|Casting|CastToPlayerShip _array_element))
        (Utilities|IsValid _asplayer_ship
          (:Is%20Valid
            (if (< (Variables|/Game/MultiplayerShip/Blueprints/PlayerShip/PlayerShip.PlayerShip_C|GetHealth _asplayer_ship) 1.0)
              (bind _asship_mode (Utilities|Casting|CastToShipMode (Game|GetGameMode)))
              (CallFunction|Respawn _asship_mode))))))))

(event EventBeginPlay
  ;[1 1 1] Store all the start points
  (Networking|SwitchHasAuthority
    (:Authority
      (bind _outactors (Actor|GetAllActorsOfClass "/Script/Engine.PlayerStart"))
      (for _array_element _outactors
        (Utilities|IsValid _array_element
          (:Is%20Valid
            (Utilities|Array|Add (Variables|Default|GetplayerStarts) _array_element)))))))

(fn ConstructionScript)

(fn GetRandomStart
  (bind _playerstarts (Variables|Default|GetplayerStarts))
  (return (Utilities|Array|Get(acopy) _playerstarts (Math|Random|RandomIntegerinRange 0 (Utilities|Array|Length _playerstarts)))))