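; Behavior tree task that moves an AI-controlled Minion along the spline of its MinionPath.
; On tick it advances a stored Distance by a fixed step, independent of delta time, and snaps the pawn to that world-space point without sweeping.
; It writes the point to the Position blackboard key, then finishes successfully after that single step.
; The execute event is empty, so all work happens in Tick.
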(event EventReceiveExecute
  (params (OwnerActor :type Actor%20Object%20Reference)))

(event EventTick
  (params (OwnerActor :type Actor%20Object%20Reference) (DeltaSeconds :type Float%20%28single-precision%29))
  (bind _asminion_aicontroller (Utilities|Casting|CastToMinionAIController OwnerActor))
  (bind _asminion (Utilities|Casting|CastToMinion (Pawn|GetControlledPawn _asminion_aicontroller)))
  (bind _output_get (Variables|Default|SetDistance (+ (Variables|Default|GetDistance) 1e+01)))
  (Transformation|SetActorLocation _asminion (Spline|GetLocationatDistanceAlongSpline (Variables|/Game/MultiplayerShip/Blueprints/MinionAI/MinionPath.MinionPath_C|GetSpline (Variables|/Game/MultiplayerShip/Blueprints/MinionAI/Minion.Minion_C|GetMinionPath _asminion)) _output_get "World") false false)
  (AI|BehaviorTree|SetBlackboardValueasVector (Variables|Default|GetPosition) (Spline|GetLocationatDistanceAlongSpline (Variables|/Game/MultiplayerShip/Blueprints/MinionAI/MinionPath.MinionPath_C|GetSpline (Variables|/Game/MultiplayerShip/Blueprints/MinionAI/Minion.Minion_C|GetMinionPath _asminion)) _output_get "World"))
  (AI|BehaviorTree|FinishExecute true))