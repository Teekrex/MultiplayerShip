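; Behavior tree service for minion AI that feeds a moving target point along the minion's spline path into the Blackboard.
; Each service tick casts to the MinionAIController and its Minion pawn, then advances a stored distance by a fixed step.
; It samples the MinionPath spline at that distance in world space and writes the location to the Point key, independently of the pawn's position.
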(event EventTick
  (params (OwnerActor :type Actor%20Object%20Reference) (DeltaSeconds :type Float%20%28single-precision%29))
  (bind _asminion_aicontroller (Utilities|Casting|CastToMinionAIController OwnerActor))
  (bind _asminion (Utilities|Casting|CastToMinion (Pawn|GetControlledPawn _asminion_aicontroller)))
  (bind _output_get (Variables|Default|SetDistance (+ (Variables|Default|GetDistance) 5e+01)))
  (AI|BehaviorTree|SetBlackboardValueasVector (Variables|Default|GetPoint) (Spline|GetLocationatDistanceAlongSpline (Variables|/Game/MultiplayerShip/Blueprints/MinionAI/MinionPath.MinionPath_C|GetSpline (Variables|/Game/MultiplayerShip/Blueprints/MinionAI/Minion.Minion_C|GetMinionPath _asminion)) _output_get "World")))